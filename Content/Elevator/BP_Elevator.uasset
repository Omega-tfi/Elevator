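; Elevator actor that starts on a random one of four evenly spaced floors and travels to the floor of the pressed button.
; Interact matches the hit component to a button and calls MoveElevator, where a timeline interpolates Z from the current height to the target.
; A press also closes every Doors actor in the level and temporarily swaps that button's material, with the Delay sitting inside the door loop.
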(event `self.ReceiveBeginPlay`
  (bind (_returnvalue_x _returnvalue_y) (`KismetMathLibrary.BreakVector` (`self.K2_GetActorLocation`)))
  (`self.K2_SetActorLocation` (`KismetMathLibrary.MakeVector` _returnvalue_x _returnvalue_y (* (`KismetMathLibrary.RandomInteger` 4) 500.0))))

(event `MoveElevator`
  (params (TargetHeight :type "Float (double-precision)"))
  (bind (_returnvalue_x _returnvalue_y _returnvalue_z) (`KismetMathLibrary.BreakVector` (`self.K2_GetActorLocation`)))
  (set `self.StartPos` _returnvalue_z)
  (set `self.Distance` (- TargetHeight _returnvalue_z))
  (bind (_direction _newtrack_0) (`Timeline|Timeline_0` :!via `PlayFromStart`)
    (:`Update`
      (`self.K2_SetActorLocation` (`KismetMathLibrary.MakeVector` _returnvalue_x _returnvalue_y (+ (`self.StartPos`) (* _newtrack_0 (`self.Distance`))))))))

(event `/Game/Elevator/BPI_Interact.Interact`
  (params (`Component Hit` :type "ActorComponent Object Reference"))
  (bind _button_0 (`self.Button 0`))
  (bind _button_1 (`self.Button 1`))
  (bind _button_2 (`self.Button 2`))
  (bind _button_3 (`self.Button 3`))
  (if (== `Component Hit` (`self.Button 0`))
    (`self.MoveElevator` 0.0)
    (bind _outactors (`GameplayStatics.GetAllActorsOfClass` "/Game/Elevator/Doors.Doors_C"))
    (for _array_element _outactors
      (bind _asdoors (cast `/Game/Elevator/Doors` _array_element))
      (`/Game/Elevator/Doors.CloseDoor` _asdoors)
      (`PrimitiveComponent.SetMaterial` _button_0 0 "/Engine/MapTemplates/Materials/BasicAsset03.BasicAsset03")
      (`KismetSystemLibrary.Delay` 2.0)
      (`PrimitiveComponent.SetMaterial` _button_0 0 "/Engine/EngineDebugMaterials/BlackUnlitMaterial.BlackUnlitMaterial"))
    (elif (== `Component Hit` (`self.Button 1`))
      (`self.MoveElevator` 500.0)
      (bind _outactors_2 (`GameplayStatics.GetAllActorsOfClass` "/Game/Elevator/Doors.Doors_C"))
      (for _array_element_2 _outactors_2
        (bind _asdoors_2 (cast `/Game/Elevator/Doors` _array_element_2))
        (`/Game/Elevator/Doors.CloseDoor` _asdoors_2)
        (`PrimitiveComponent.SetMaterial` _button_1 0 "/Engine/MapTemplates/Materials/BasicAsset03.BasicAsset03")
        (`KismetSystemLibrary.Delay` 2.0)
        (`PrimitiveComponent.SetMaterial` _button_1 0 "/Engine/EngineDebugMaterials/BlackUnlitMaterial.BlackUnlitMaterial"))
      (elif (== `Component Hit` (`self.Button 2`))
        (`self.MoveElevator` 1000.0)
        (bind _outactors_3 (`GameplayStatics.GetAllActorsOfClass` "/Game/Elevator/Doors.Doors_C"))
        (for _array_element_3 _outactors_3
          (bind _asdoors_3 (cast `/Game/Elevator/Doors` _array_element_3))
          (`/Game/Elevator/Doors.CloseDoor` _asdoors_3)
          (`PrimitiveComponent.SetMaterial` _button_2 0 "/Engine/MapTemplates/Materials/BasicAsset03.BasicAsset03")
          (`KismetSystemLibrary.Delay` 2.0)
          (`PrimitiveComponent.SetMaterial` _button_2 0 "/Engine/EngineDebugMaterials/BlackUnlitMaterial.BlackUnlitMaterial"))
        (elif (== `Component Hit` (`self.Button 3`))
          (`self.MoveElevator` 1500.0)
          (bind _outactors_4 (`GameplayStatics.GetAllActorsOfClass` "/Game/Elevator/Doors.Doors_C"))
          (for _array_element_4 _outactors_4
            (bind _asdoors_4 (cast `/Game/Elevator/Doors` _array_element_4))
            (`/Game/Elevator/Doors.CloseDoor` _asdoors_4)
            (`PrimitiveComponent.SetMaterial` _button_3 0 "/Engine/MapTemplates/Materials/BasicAsset03.BasicAsset03")
            (`KismetSystemLibrary.Delay` 2.0)
            (`PrimitiveComponent.SetMaterial` _button_3 0 "/Engine/EngineDebugMaterials/BlackUnlitMaterial.BlackUnlitMaterial")))))))

(fn `UserConstructionScript`)